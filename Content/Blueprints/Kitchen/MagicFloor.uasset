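; MagicFloor is a kitchen floor actor that shuttles back and forth on its own, pausing briefly after each move.
; Tick uses the ReadyCheck flag to start the Move timeline once per cycle, in reverse or forward depending on FloorMoving.
; Timeline updates add a forward or backward vector track as an unswept local offset, accumulating movement each update.
; When it finishes, a delay precedes flipping FloorMoving and clearing ReadyCheck.
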(event `self.ReceiveTick`
  (params (DeltaSeconds :type "Float (single-precision)"))
  (if (not (`self.readyCheck`))
    (set `self.readyCheck` true)
    (if (`self.FloorMoving`)
      (bind (_direction _movefloor _movefloorback) (`Timeline|Move` :!via `Reverse` :!label _label)
        (:`Update`
          (if (`self.FloorMoving`)
            (`self.K2_AddActorLocalOffset` _movefloorback)
            (else
              (`self.K2_AddActorLocalOffset` _movefloor))))
        (:`Finished`
          (`KismetSystemLibrary.Delay` 2.0)
          (if (`self.FloorMoving`)
            (set `self.FloorMoving` false)
            (set `self.readyCheck` false)
            (else
              (set `self.FloorMoving` true)
              (set `self.readyCheck` false)))))
      (else
        (goto _label)))))

(fn `UserConstructionScript`)