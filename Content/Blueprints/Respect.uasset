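; Respect is an interactable actor that plays audio while a MOOnshineWorksCharacter is inside its overlap area.
; Begin overlap caches the character and starts the Audio1 component if it is not already playing, and end overlap stops it.
; OnInteract plays the Death04 sound attached to the cached character's mesh.
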(event `self.OnInteract`
  (params (Target :type "Actor Object Reference"))
  (`GameplayStatics.PlaySoundAttached` "/Game/Sounds/Death/Death04.Death04" (`Character.Mesh` (stale `self.ReceiveActorBeginOverlap` _asmoonshine_works_character))))

(event `self.ReceiveActorBeginOverlap`
  (params (OtherActor :type "Actor Object Reference"))
  (bind _audio1 (`self.Audio1`))
  (bind _asmoonshine_works_character (cast `MOOnshineWorksCharacter` OtherActor))
  (bind _returnvalue (`AudioComponent.IsPlaying` _audio1))
  (if (not _returnvalue)
    (`AudioComponent.Play` _audio1 0.0)))

(event `self.ReceiveActorEndOverlap`
  (params (OtherActor :type "Actor Object Reference"))
  (bind _audio1 (`self.Audio1`))
  (cast `MOOnshineWorksCharacter` OtherActor)
  (bind _returnvalue (`AudioComponent.IsPlaying` _audio1))
  (if _returnvalue
    (`AudioComponent.Stop` _audio1)))

(fn `UserConstructionScript`)