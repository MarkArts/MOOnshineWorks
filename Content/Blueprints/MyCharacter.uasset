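; Player character Blueprint that handles the HUD, pause menu and audio-visual feedback for movement, damage and death.
; BeginPlay adds the HUD and settings widgets, while Escape, Enter or gamepad Special Right toggles pause.
; Tick requests walk or run sounds every grounded moving frame, with further cues on jump and landing.
; Damage briefly flashes a hit glow; death shows a game-over screen, disables input, then opens the EVERYTHING level.
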(event `self.ReceiveBeginPlay`
  ;[1 1 1] On start: Start Bg music and create hud widget
  (`|ExecutionSequence`
    (:`then_0`
      (bind _returnvalue (`|CreateWidget` "/Game/Blueprints/HUDBlueprints/HudWidget.HUDWidget_C"))
      (`UserWidget.AddToViewport` _returnvalue))
    (:`then_1`
      ;[1 1 1] Will be fired to load graphic settings, removes itself after loading
      (bind _returnvalue_2 (`|CreateWidget` "/Game/Blueprints/HUDBlueprints/Settings/SettingsScreen.SettingsScreen_C"))
      (`UserWidget.AddToViewport` _returnvalue_2))))

(event `Key|Escape` :paused true
  (bind _returnvalue (`GameplayStatics.GetPlayerController` 0))
  ;[1 1 1] Assign pause menu to keys
  (:`Pressed`
    (if (`GameplayStatics.IsGamePaused`) :!label _label
      (`GameplayStatics.SetGamePaused` false)
      (`Widget.RemoveFromParent` (stale _returnvalue_2))
      (set `PlayerController.bShowMouseCursor` false _returnvalue)
      (else
        (`GameplayStatics.SetGamePaused` true)
        (bind _returnvalue_2 (`|CreateWidget` "/Game/Blueprints/HUDBlueprints/PauseMenu.PauseMenu_C"))
        (`UserWidget.AddToViewport` _returnvalue_2)
        (`self.EnableInput` _returnvalue)
        (set `PlayerController.bShowMouseCursor` true _returnvalue)))))

(event `Key|Enter` :paused true
  ;[1 1 1] Assign pause menu to keys
  (:`Pressed`
    (goto _label)))

(event `Key|Gamepad_Special_Right` :paused true
  ;[1 1 1] Assign pause menu to keys
  (:`Pressed`
    (goto _label)))

(event `self.ReceiveTick`
  (params (DeltaSeconds :type "Float (single-precision)"))
  (bind _mesh (`self.Mesh`))
  ;[1 1 1] Tick event for sounds walk & run
  (if (`NavMovementComponent.IsFalling` (`self.GetMovementComponent` (`GameplayStatics.GetPlayerCharacter` 0)))
    _
    (elif (or (`self.IsMovingForward`) (`self.IsMovingSideway`))
      (if (`self.IsSprinting`)
        (`GameplayStatics.PlaySoundAttached` "/Game/Sounds/CharacterRun/RunCue.RunCue" _mesh)
        (else
          (`GameplayStatics.PlaySoundAttached` "/Game/Sounds/CharacterWalk/WalkSoundCue.WalkSoundCue" _mesh))))))

(event `self.OnLanded`
  (params (Hit :type "EngineTypes.HitResult Structure (by ref)"))
  ;[1 1 1] Play sounds on deal damage, landing or jumping
  (`GameplayStatics.PlaySoundAttached` "/Game/Sounds/Landing/LandingCue.LandingCue" (`self.Mesh`)))

(event `InputAction|Jump` :overrideparent false
  ;[1 1 1] Play sounds on deal damage, landing or jumping
  (:`Pressed`
    (if (not (`NavMovementComponent.IsFalling` (`self.GetMovementComponent` (`GameplayStatics.GetPlayerCharacter` 0))))
      (`GameplayStatics.PlaySoundAttached` "/Game/Sounds/Jump/JumpCue.JumpCue" (`self.Mesh`)))))

(event `self.OnDealDamage`
  (params (Damage :type "Float (single-precision)"))
  ;[1 1 1] Play sounds on deal damage, landing or jumping
  (`GameplayStatics.PlaySoundAttached` "/Game/Sounds/TakenDamage/TakenDamageCue.TakenDamageCue" (`self.Mesh`))
  (bind _returnvalue (`|CreateWidget` "/Game/Blueprints/HUDBlueprints/HitGlow.HitGlow_C"))
  (`UserWidget.AddToViewport` _returnvalue)
  (`UserWidget.PlayAnimation` _returnvalue (`/Game/Blueprints/HUDBlueprints/HitGlow.FadeIn` _returnvalue))
  (`KismetSystemLibrary.Delay` 0.25)
  (`Widget.RemoveFromParent` _returnvalue))

(event `self.OnDie`
  ;[1 1 1] OnDie Event - Play sounds, show gameover screen, open new level
  (`GameplayStatics.PlaySoundAttached` "/Game/Sounds/Death/DeathCUe.DeathCue" (`self.Mesh`))
  (`KismetSystemLibrary.Delay` 1.0)
  (bind _returnvalue (`|CreateWidget` "/Game/Blueprints/HUDBlueprints/GameOverScreen.GameOverScreen_C"))
  (`UserWidget.AddToViewport` _returnvalue)
  (`UserWidget.PlayAnimation` _returnvalue (`/Game/Blueprints/HUDBlueprints/GameOverScreen.FadeAnim` _returnvalue))
  (`self.DisableInput` null)
  (`KismetSystemLibrary.Delay` 7.5)
  (`Widget.RemoveFromParent` _returnvalue)
  (`GameplayStatics.OpenLevel` "EVERYTHING"))

(fn `UserConstructionScript`)