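; BP_Shotgun is the shotgun gun Blueprint, handling visual and audio feedback for firing and charging.
; Use plays the shoot animation and sound, layering an extra cue when Charge is exactly full.
; Charge start plays the charge animation, activates charge and smoke particles and sequences audio with fades, while charge end deactivates particles and fades out playing audio.
; The construction script positions both particle systems at mesh sockets.
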(event `self.SetVisibility`
  (params (Visible :type Boolean))
  (`SceneComponent.SetVisibility` (`self.SkeletalMesh1`) Visible false))

(event `self.OnUse`
  (bind _skeletalmesh1 (`self.SkeletalMesh1`))
  (`|ExecutionSequence`
    (:`then_0`
      (`GameplayStatics.PlaySoundAttached` "/Game/Sounds/Shoot/Shotgun/ShotgunShootCue.ShotgunShootCue" _skeletalmesh1)
      (if (== (`self.Charge`) 1.0)
        (`GameplayStatics.PlaySoundAttached` "/Game/Sounds/Shoot/ShootCharged/ChargedShotCue.ChargedShotCue" (`self.SkeletalMesh1`))))
    (:`then_1`
      (`SkeletalMeshComponent.PlayAnimation` _skeletalmesh1 "/Game/BP_Meshes/Shotgun/Animation/Shotgun_Shoot.Shotgun_Shoot" false))))

(event `self.OnStartCharge`
  (bind _chargeparticlesystem (`self.ChargeParticleSystem`))
  (`|ExecutionSequence`
    (:`then_0`
      (`ActorComponent.SetActive` _chargeparticlesystem true true)
      (`ParticleSystemComponent.GenerateParticleEvent` _chargeparticlesystem "None" 0.0 (0.0 0.0 0.0) (0.0 0.0 0.0) (0.0 0.0 0.0) :!label _label))
    (:`then_1`
      (`SkeletalMeshComponent.PlayAnimation` (`self.SkeletalMesh1`) "/Game/BP_Meshes/Shotgun/Animation/Shotgun_Charge.Shotgun_Charge" false))
    (:`then_2`
      (`AudioComponent.Play` 0.0)
      (`AudioComponent.FadeIn` 4.0 1.0 2.0)
      (`KismetSystemLibrary.Delay` 1.5)
      (`AudioComponent.FadeOut` 1.5))
    (:`then_3`
      (`ActorComponent.SetActive` (`self.SmokeParticleSystem`) true false))))

(event `self.OnEndCharge`
  (`|ExecutionSequence`
    (:`then_0`
      (`ActorComponent.SetActive` (`self.ChargeParticleSystem`) false true)
      (goto _label))
    (:`then_1`
      (bind _returnvalue (`AudioComponent.IsPlaying`))
      (if _returnvalue
        (`AudioComponent.FadeOut` 0.75)))
    (:`then_2`
      (bind _returnvalue_2 (`AudioComponent.IsPlaying`))
      (if _returnvalue_2
        (`AudioComponent.FadeOut` 0.75)))
    (:`then_3`
      (`ActorComponent.SetActive` (`self.SmokeParticleSystem`) false false))))

(fn `UserConstructionScript`
  (bind _skeletalmesh1 (`self.SkeletalMesh1`))
  (`SceneComponent.K2_SetWorldLocation` (`self.ChargeParticleSystem`) (`SceneComponent.GetSocketLocation` _skeletalmesh1 "BulletSpawn") false)
  (`SceneComponent.K2_SetWorldLocation` (`self.SmokeParticleSystem`) (`SceneComponent.GetSocketLocation` _skeletalmesh1 "SmokePS") false))