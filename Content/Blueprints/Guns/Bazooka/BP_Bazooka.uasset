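; BP_Bazooka is a bazooka weapon Blueprint that handles the gun's visibility, animation, sound and charge particles.
; Charge start plays the charge animation, activates the particle system and layers audio with timed fades.
; Charge end deactivates the particles and fades out playing audio, while use plays the shot sound and shoot animation.
; The construction script snaps the charge particles to the mesh's BulletSpawn socket.
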(event `self.SetVisibility`
  (params (Visible :type Boolean))
  (`SceneComponent.SetVisibility` (`self.SkeletalMesh1`) Visible false))

(event `self.OnUse`
  (bind _skeletalmesh1 (`self.SkeletalMesh1`))
  (`|ExecutionSequence`
    (:`then_0`
      (`GameplayStatics.PlaySoundAttached` "/Game/Sounds/Shoot/ShootCharged/ChargedShotCue.ChargedShotCue" _skeletalmesh1))
    (:`then_1`
      (`SkeletalMeshComponent.PlayAnimation` _skeletalmesh1 "/Game/BP_Meshes/Bazooka/Animation/Bazooka_Shoot.Bazooka_Shoot" false))))

(event `self.OnStartCharge`
  (bind _chargeparticlesystem (`self.ChargeParticleSystem`))
  (`|ExecutionSequence`
    (:`then_0`
      (`SkeletalMeshComponent.PlayAnimation` (`self.SkeletalMesh1`) "/Game/BP_Meshes/Bazooka/Animation/Bazooka_Charge.Bazooka_Charge" false))
    (:`then_1`
      (`ActorComponent.SetActive` _chargeparticlesystem true true)
      (`ParticleSystemComponent.GenerateParticleEvent` _chargeparticlesystem "None" 0.0 (0.0 0.0 0.0) (0.0 0.0 0.0) (0.0 0.0 0.0) :!label _label))
    (:`then_2`
      (`AudioComponent.Play` 0.0)
      (`AudioComponent.FadeIn` 4.0 1.0 2.5)
      (`KismetSystemLibrary.Delay` 3.0)
      (`AudioComponent.FadeOut` 1.0))))

(event `self.OnEndCharge`
  (`|ExecutionSequence`
    (:`then_0`
      (`ActorComponent.SetActive` (`self.ChargeParticleSystem`) false true)
      (goto _label))
    (:`then_1`
      (bind _returnvalue (`AudioComponent.IsPlaying`))
      (if _returnvalue
        (`AudioComponent.FadeOut` 0.5)))
    (:`then_2`
      (bind _returnvalue_2 (`AudioComponent.IsPlaying`))
      (if _returnvalue_2
        (`AudioComponent.FadeOut` 0.5)))))

(fn `UserConstructionScript`
  (`SceneComponent.K2_SetWorldLocation` (`self.ChargeParticleSystem`) (`SceneComponent.GetSocketLocation` (`self.SkeletalMesh1`) "BulletSpawn") false))