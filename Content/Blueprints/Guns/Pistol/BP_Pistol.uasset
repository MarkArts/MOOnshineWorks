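; Pistol weapon Blueprint that supplies the audiovisual feedback for shooting and charging, using crossbow animations on its skeletal mesh.
; Use plays the shoot sound and animation, layering a charged-shot cue when Charge is exactly full.
; Charge start and end toggle a particle system and fire a particle event, with start also playing the charge animation.
; The construction script places those particles at the BulletSpawn socket.
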(event `self.SetVisibility`
  (params (Visible :type Boolean))
  (`SceneComponent.SetVisibility` (`self.SkeletalMesh1`) Visible false))

(event `self.OnUse`
  (bind _skeletalmesh1 (`self.SkeletalMesh1`))
  (`|ExecutionSequence`
    (:`then_0`
      (`GameplayStatics.PlaySoundAttached` "/Game/Sounds/Shoot/Crossbow/ShootCue.ShootCue" _skeletalmesh1)
      (if (== (`self.Charge`) 1.0)
        (`GameplayStatics.PlaySoundAttached` "/Game/Sounds/Shoot/ShootCharged/ChargedShotCue.ChargedShotCue" (`self.SkeletalMesh1`))))
    (:`then_1`
      (`SkeletalMeshComponent.PlayAnimation` _skeletalmesh1 "/Game/BP_Meshes/Pistol/Animation/Crossbow_animation_shoot.Crossbow_animation_shoot" false))))

(event `self.OnStartCharge`
  (bind _chargeparticlesystem (`self.ChargeParticleSystem`))
  (`ActorComponent.SetActive` _chargeparticlesystem true true)
  (`|ExecutionSequence`
    (:`then_0`
      (`ParticleSystemComponent.GenerateParticleEvent` _chargeparticlesystem "None" 0.0 (0.0 0.0 0.0) (0.0 0.0 0.0) (0.0 0.0 0.0) :!label _label))
    (:`then_1`
      (`SkeletalMeshComponent.PlayAnimation` (`self.SkeletalMesh1`) "/Game/BP_Meshes/Pistol/Animation/Crossbow_animation_charge.Crossbow_animation_charge" false))))

(event `self.OnEndCharge`
  (`ActorComponent.SetActive` (`self.ChargeParticleSystem`) false true)
  (goto _label))

(fn `UserConstructionScript`
  (`SceneComponent.K2_SetWorldLocation` (`self.ChargeParticleSystem`) (`SceneComponent.GetSocketLocation` (`self.SkeletalMesh1`) "BulletSpawn") false))