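; Door actor that swings open and closed about its yaw axis, toggling each time its DoorOpen event is called.
; BeginPlay caches the actor's starting rotation, and the DoorClosed flag decides whether the DoorOpening timeline plays forward or reverses.
; Each timeline update combines that starting rotation with the DoorRot yaw and sets it as the actor's relative rotation, without sweep.
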(event `self.DoorOpen`
  (if (`self.DoorClosed`)
    (set `self.DoorClosed` false)
    (bind (_direction _doorrot) (`Timeline|DoorOpening` :!label _label)
      (:`Update`
        (`self.SetActorRelativeRotation` (`KismetMathLibrary.ComposeRotators` (`self.BeginningRot`) (`KismetMathLibrary.MakeRot` 0.0 _doorrot)))))
    (else
      (set `self.DoorClosed` true)
      (goto _label :!via `Reverse`))))

(event `self.ReceiveBeginPlay`
  (set `self.BeginningRot` (`self.K2_GetActorRotation`)))

(fn `UserConstructionScript`)