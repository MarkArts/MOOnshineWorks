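; Basement door actor that swings open or shut around its yaw axis when its DoorOpen event fires.
; BeginPlay caches the starting rotation, and the DoorOpening timeline adds its yaw track to that base on each update.
; The DoorClosed flag selects playing the timeline with an unlock sound or reversing it with a close sound, though this graph never sets that flag.
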(event `self.DoorOpen`
  (bind _staticmesh1 (`self.StaticMesh1`))
  (if (`self.DoorClosed`)
    (`GameplayStatics.PlaySoundAttached` "/Game/Sounds/Door/Unlock/UnlockCue.UnlockCue" _staticmesh1)
    (bind (_direction _doorrot) (`Timeline|DoorOpening` :!label _label)
      (:`Update`
        (`self.K2_SetActorRelativeRotation` (`KismetMathLibrary.ComposeRotators` (`self.BeginningRot`) (`KismetMathLibrary.MakeRot` 0.0 _doorrot)))))
    (else
      (`GameplayStatics.PlaySoundAttached` "/Game/Sounds/Door/CloseDoor/CloseDoorCue.CloseDoorCue" _staticmesh1)
      (goto _label :!via `Reverse`))))

(event `self.ReceiveBeginPlay`
  (set `self.BeginningRot` (`self.K2_GetActorRotation`)))

(fn `UserConstructionScript`)