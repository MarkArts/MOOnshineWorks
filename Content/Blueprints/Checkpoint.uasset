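; Interactable checkpoint Blueprint that creates a checkpoint for the MOOnshineWorks character when that character interacts with it.
; OnInteract casts the target to the character class and passes it to CreateCheckpoint.
; While the checkpoint is unused, its activation sphere switches a spotlight on when the character enters and off when it leaves.
; A used checkpoint turns the spotlight on at BeginPlay and ignores overlaps.
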(event `self.OnInteract`
  (params (Target :type "Actor Object Reference"))
  (bind _asmoonshineworkscharacter (cast `MOOnshineWorksCharacter` Target))
  (`Helpers.CreateCheckpoint` _asmoonshineworkscharacter))

(event `self.ReceiveBeginPlay`
  (if (`self.IsUsed`)
    (`SceneComponent.SetVisibility` (`self.SpotLight1`) true false :!label _label)))

(event `self.Activation Sphere.OnComponentBeginOverlap`
  (params (OtherActor :type "Actor Object Reference") (OtherComp :type "PrimitiveComponent Object Reference") (OtherBodyIndex :type Integer) (bFromSweep :type Boolean) (SweepResult :type "EngineTypes.HitResult Structure (by ref)"))
  (if (not (`self.IsUsed`))
    (cast `MOOnshineWorksCharacter` OtherActor)
    (goto _label)))

(event `self.Activation Sphere.OnComponentEndOverlap`
  (params (OtherActor :type "Actor Object Reference") (OtherComp :type "PrimitiveComponent Object Reference") (OtherBodyIndex :type Integer))
  (if (not (`self.IsUsed`))
    (cast `MOOnshineWorksCharacter` OtherActor)
    (`SceneComponent.SetVisibility` (`self.SpotLight1`) false false)))

(fn `UserConstructionScript`)